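; BP_ItemBase is a base actor for inventory items placed in the world, driven by a data table row.
; On construction and BeginPlay, it looks up its row name in DT_Items, caches the item data and applies that row's mesh, so placed items preview in the editor.
; Its InteractWithItem function stores the interacting player reference and returns the item data flagged as valid.
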(event Custom|UpdateItemActor
  (bind _returnvalue (Utilities|GetDataTableRow "/Game/Blueprints/Inventory/DT_Items.DT_Items" (Variables|Default|GetDatatableItemNumber))
    (:then
      (Variables|Default|SetItemData _returnvalue)
      (Components|StaticMesh|SetStaticMesh (Variables|Default|GetItemMesh) (.mesh (Variables|Default|GetItemData))))))

(event EventBeginPlay
  (CallFunction|UpdateItemActor))

(fn ConstructionScript
  (CallFunction|UpdateItemActor))

(fn InteractwithItem
  (params (PlayerRef :type BP%20First%20Person%20Character%20Object%20Reference))
  (Variables|Default|SetPlayer%20Ref PlayerRef)
  (return (Variables|Default|GetItemData) true))